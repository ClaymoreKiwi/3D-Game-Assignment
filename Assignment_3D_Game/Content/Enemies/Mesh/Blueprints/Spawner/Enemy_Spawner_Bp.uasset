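; Enemy spawner actor that continuously produces waves of enemies for the player to deal with.
; On BeginPlay it triggers a custom spawn event that spawns a configurable number of the chosen enemy class at the spawner's transform.
; The event then waits for a configurable delay and calls itself again with the spawner's current transform, repeating with no stop condition.
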(event `self.ReceiveBeginPlay`
  ;[1 1 1] Continuously spawn enemies for the player to deal with
  (`self.Spawn_E` (`self.Enemy`) (`self.GetTransform`) (`self.Num Enemies`)))

(event `Spawn_E`
  (params (Enemy :type "Actor Class Reference") (SpawnTransform :type "Transform Structure") (Num_Enemies :type Integer))
  ;[1 1 1] Continuously spawn enemies for the player to deal with
  (for _ (range Num_Enemies)
    (`|SpawnActorFromClass` Enemy SpawnTransform "Undefined" "OverrideRootScale" null null))
  (`KismetSystemLibrary.Delay` (`self.Spawn_Delay`))
  (`self.Spawn_E` (`self.Enemy`) (`self.GetTransform`) (`self.Num Enemies`)))

(fn `UserConstructionScript`)