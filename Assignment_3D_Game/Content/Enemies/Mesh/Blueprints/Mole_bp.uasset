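; Mole enemy character that chases the player and awards points when shot dead.
; On BeginPlay it picks one of three random walk speeds and starts an AI MoveTo toward Player1, reissued on success or failure.
; Bullet hits on the capsule reduce Health and play a hit montage; at zero it is destroyed after a delay and adds to Player1's Points.
; Tick stops movement and disables collision once Health drops below one.
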(event `self.ReceiveTick`
  (params (DeltaSeconds :type "Float (single-precision)"))
  ;[1 1 1] Setting movement and collision boxes to non interactable
  (if (< (`self.Health`) 1.0)
    (set `CharacterMovementComponent.MaxWalkSpeed` 0.0 (`self.CharacterMovement`))
    (`PrimitiveComponent.SetCollisionEnabled` (`self.CapsuleComponent`) "NoCollision")
    (`PrimitiveComponent.SetCollisionEnabled` (`self.FPS_HB`) "NoCollision")
    (`PrimitiveComponent.SetCollisionEnabled` (`self.Mesh`) "NoCollision")))

(event `self.ReceiveBeginPlay`
  ;[1 1 1] Basic AI Nav Mesh Settup
  (bind _asplayer_1 (cast `/Game/Player/Mesh/Player1` (`GameplayStatics.GetPlayerCharacter` 0)))
  (bind _output_get (set `self.Player1_Ref` _asplayer_1))
  (`self.Chase Player` _output_get)
  (set `CharacterMovementComponent.MaxWalkSpeed` (select `int` (`KismetMathLibrary.RandomInteger` 3) :`0` 300.0 :`1` 400.0 :`2` 500.0 :!type "Float (single-precision)") (`self.CharacterMovement`)))

(event `Chase Player`
  (params (Player :type "/Game/Player/Mesh/Player1 Object Reference"))
  ;[1 1 1] Basic AI Nav Mesh Settup
  (`|AIMoveTo` self (0.0 0.0 0.0) Player (`self.Acceptance Radius`)
    (:`OnSuccess`
      _)
    (:`OnFail`
      _))
  (`self.Chase Player` (`self.Player1_Ref`)))

(event `self.CapsuleComponent.OnComponentHit`
  (params (HitComponent :type "PrimitiveComponent Object Reference") (OtherActor :type "Actor Object Reference") (OtherComp :type "PrimitiveComponent Object Reference") (NormalImpulse :type "Vector Structure") (Hit :type "HitResult Structure (by ref)"))
  (bind _player1_ref (`self.Player1_Ref`))
  ;[1 1 1] Enemy Damage & hit animation sequence
  (cast `/Game/Props/Weapons/Bullet_bp` OtherActor)
  (bind _output_get (set `self.Health` (- (`self.Health`) 10.0)))
  (if (<= _output_get 0.0)
    (`self.PlayAnimMontage` "/Game/Enemies/Animations/Rig_Hit_Montage.Rig_Hit_Montage")
    (`KismetSystemLibrary.Delay` 2.0)
    (`self.K2_DestroyActor`)
    (set `/Game/Player/Mesh/Player1.Points` (+ (`/Game/Player/Mesh/Player1.Points` _player1_ref) 10) _player1_ref)
    (else
      (`self.PlayAnimMontage` "/Game/Enemies/Animations/Rig_Hit_Montage.Rig_Hit_Montage"))))

(fn `UserConstructionScript`)