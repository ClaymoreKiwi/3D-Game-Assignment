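; LoadNexLevel is a trigger actor that advances the player to the next level once they have enough points.
; When a Player1 overlaps its NextLevel component, it compares Points against NextLevelPoints and calls LoadLevel on the player's game instance with LevelName.
; If TurnMusicOff is set, it also stops RandomSong on GameInstance_MenuToLevel1.
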(event `self.ReceiveBeginPlay`)

(event `self.Next Level.OnComponentBeginOverlap`
  (params (OverlappedComponent :type "PrimitiveComponent Object Reference") (OtherActor :type "Actor Object Reference") (OtherComp :type "PrimitiveComponent Object Reference") (OtherBodyIndex :type Integer) (bFromSweep :type Boolean) (SweepResult :type "HitResult Structure (by ref)"))
  ;[1 1 1] Open Next Level Based off of player points
  (bind _asplayer_1 (cast `/Game/Player/Mesh/Blueprints/Player1` OtherActor))
  (if (>= (`/Game/Player/Mesh/Blueprints/Player1.Points` _asplayer_1) (`self.NextLevelPoints`))
    (`/Game/Levels/Blueprints/GameInstance_MenuToLevel1.LoadLevel` (`/Game/Player/Mesh/Blueprints/Player1.GetGameInst` _asplayer_1) (`self.Level Name`) _asplayer_1)
    (if (`self.TurnMusicOff`)
      (bind _asgame_instance_menu_to_level_1 (cast `/Game/Levels/Blueprints/GameInstance_MenuToLevel1` (`GameplayStatics.GetGameInstance`)))
      (`AudioComponent.Stop` (`/Game/Levels/Blueprints/GameInstance_MenuToLevel1.Random Song` _asgame_instance_menu_to_level_1)))))

(fn `UserConstructionScript`)