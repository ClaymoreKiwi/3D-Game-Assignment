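; Game instance that carries player state and background music across level transitions, named for the menu-to-Level 1 flow.
; LoadLevel snapshots the player's points, reserved ammo, clip ammo and current health, sets a transition flag, then opens the named level.
; PlayBackgroundMusic creates a 2D sound with optional persistence across level loads, stores it and plays it.
; Restoring the saved values is not handled here.
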(event `LoadLevel`
  (params (`Level To Load` :type Name) (Player :type "/Game/Player/Mesh/Blueprints/Player1 Object Reference"))
  (`self.GatherPlayerState` Player)
  (set `self.ShouldTransition` true)
  (`GameplayStatics.OpenLevel` `Level To Load`))

(fn `GatherPlayerState`
  (params (Player :type "/Game/Player/Mesh/Blueprints/Player1 Object Reference"))
  (set `self.Player_Points` (`/Game/Player/Mesh/Blueprints/Player1.Points` Player))
  (set `self.Player_Ammo_To_Reload` (`/Game/Player/Mesh/Blueprints/Player1.Total_Ammo_Reserved` Player))
  (set `self.Ammo_In_Clip` (`/Game/Player/Mesh/Blueprints/Player1.Ammo_In_Clip` Player))
  (set `self.Current_Health` (`/Game/Player/Mesh/Blueprints/Player1.Health_Current` Player)))

(fn `Play Background Music`
  (params (Sound :type "SoundBase Object Reference") (VolumeMultiplier :type "Float (double-precision)") (bPersistAcrossLevelTransition :type Boolean))
  (locals (PlayerScore :type Integer))
  (bind _returnvalue (`GameplayStatics.CreateSound2D` Sound VolumeMultiplier 1.0 0.0 null bPersistAcrossLevelTransition))
  (bind _output_get (set `self.Random Song` _returnvalue))
  (`AudioComponent.Play` _output_get 0.0))